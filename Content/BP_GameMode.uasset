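; Game mode Blueprint that scatters candlestick pickups across random spawn points when play begins.
; SpawnItem gathers all BP_SpawnPoint actors, then loops a fixed number of times, spawning a BP_Candlestick at a randomly picked point's location.
; Each used point is removed from the local list and destroyed, so no two candlesticks share a spot.
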(event `self.ReceiveBeginPlay`
  (`self.SpawnItem`))

(fn `SpawnItem`
  (locals (LocalSpawnPoints :type "Array of /Game/Character/BP_SpawnPoint Object Reference") (`Local Item` :type "/Game/Character/BP_SpawnPoint Object Reference"))
  (bind _outactors (`GameplayStatics.GetAllActorsOfClass` "/Game/Character/BP_SpawnPoint.BP_SpawnPoint_C"))
  (set `local.LocalSpawnPoints` _outactors)
  ;[1 1 1] how many items are needed - 1
  (for _ (range 5)
    (set `local.Local Item` (`KismetArrayLibrary.Array_Random` (`local.LocalSpawnPoints`)))
    (`|SpawnActorFromClass` "/Game/KTInteractionPropVol2/Blueprints/BP_Candlestick.BP_Candlestick_C" (`KismetMathLibrary.MakeTransform` (`self.K2_GetActorLocation` (`local.Local Item`))) "AdjustIfPossibleButAlwaysSpawn" "MultiplyWithRoot" null null)
    ;[1 1 1] make sure dont spawn in same spot
    (`KismetArrayLibrary.Array_RemoveItem` (`local.LocalSpawnPoints`) (`local.Local Item`))
    (`self.K2_DestroyActor` (`local.Local Item`))))

(fn `UserConstructionScript`)